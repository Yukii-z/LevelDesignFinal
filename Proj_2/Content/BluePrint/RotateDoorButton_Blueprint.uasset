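; Blueprint that rotates a referenced Door actor while the player character's RotateDoorStart flag is set.
; Each Tick it casts the player pawn to MyPlayerCharacter and polls that flag, then applies opposing local and world yaw increments plus a zero world offset.
; The per-frame steps are not scaled by delta time.
; On first activation it destroys the RotatingDoorHint actor, guarded by a one-time boolean.
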(event `self.ReceiveTick`
  (params (DeltaSeconds :type "Float (single-precision)"))
  (bind _door (`self.Door`))
  (bind _asmy_player_character (cast `/Game/MyPlayerCharacter` (`GameplayStatics.GetPlayerPawn` 0)))
  (set `self.ButtonPressed` (`/Game/MyPlayerCharacter.RotateDoorStart` _asmy_player_character))
  (if (`self.ButtonPressed`)
    (`self.K2_AddActorLocalRotation` _door (struct :`Yaw` -3.0) false false)
    (`self.K2_AddActorWorldRotation` _door (struct :`Yaw` 1.0) false false)
    (`self.K2_AddActorWorldOffset` _door (0.0 0.0 0.0) false false)
    (if (not (`self.Destoryed`))
      (`self.K2_DestroyActor` (`self.RotatingDoorHint`))
      (set `self.Destoryed` true))))

(fn `UserConstructionScript`)
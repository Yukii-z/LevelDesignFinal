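; A one-shot trigger actor that starts the game when the player first overlaps it.
; On overlap it flags the MyPlayerCharacter as game-started, sets an alarm-reaction line as player dialogue and starts that text's disappearance countdown.
; It also reveals two spotlights and hides a third, then sets a Triggered flag so it never fires again.
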(event `self.ReceiveActorBeginOverlap`
  (params (OtherActor :type "Actor Object Reference"))
  (if (not (`self.Triggered`))
    (bind _asmy_player_character (cast `/Game/MyPlayerCharacter` OtherActor))
    (set `/Game/MyPlayerCharacter.GameStart` true _asmy_player_character)
    (set `/Game/MyPlayerCharacter.PlayerTalk` "Stupid Alarm! I should probably be faster." _asmy_player_character)
    (set `/Game/MyPlayerCharacter.WordOnCountingDown` (`/Game/MyPlayerCharacter.WordDisappeartime` _asmy_player_character) _asmy_player_character)
    (set `/Game/MyPlayerCharacter.WordCountDown` true _asmy_player_character)
    (`SceneComponent.SetHiddenInGame` (`self.SpotLight`) false false)
    (`SceneComponent.SetHiddenInGame` (`self.SpotLight1`) false false)
    (`SceneComponent.SetHiddenInGame` (`self.SpotLight2`) true false)
    (set `self.Triggered` true)))

(fn `UserConstructionScript`)